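; BP_Shop is a shop actor that shows or hides a UI widget when interacted with.
; BeginPlay creates a WB_UI widget and caches it along with the player's BP_FirstPersonCharacter.
; Interact reads the character's Islooking flag, adding the widget and showing the mouse cursor when false, or removing it and hiding the cursor when true.
; The flag is only read here, never set.
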(event `self.ReceiveBeginPlay`
  (bind _returnvalue (`|CreateWidget` "/Game/WB_UI.WB_UI_C"))
  (set `self.NewVar` _returnvalue)
  (bind _asbp_first_person_character (cast `/Game/FirstPerson/Blueprints/BP_FirstPersonCharacter` (`GameplayStatics.GetPlayerCharacter` 0)))
  (set `self.As BP First Person Character` _asbp_first_person_character))

(event `/Game/BPI_Interact.interact`
  (bind _newvar (`self.NewVar`))
  (if (not (`/Game/FirstPerson/Blueprints/BP_FirstPersonCharacter.Islooking` (`self.As BP First Person Character`)))
    (`UserWidget.AddToViewport` _newvar 0)
    (set `PlayerController.bShowMouseCursor` true (`GameplayStatics.GetPlayerController` 0))
    (else
      (`Widget.RemoveFromParent` _newvar)
      (set `PlayerController.bShowMouseCursor` false (`GameplayStatics.GetPlayerController` 0)))))

(fn `UserConstructionScript`)